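; BP_Roket is a rocket actor that explodes on overlap and expires on a short lifespan if it hits nothing.
; On overlap it damages any other actor, credited to the first player controller, and spawns an explosion sound and particle effect.
; It then calls GameCheak on BP_GameMode and destroys itself, which happens only if that game mode cast succeeds.
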(event `self.ReceiveBeginPlay`
  (`self.SetLifeSpan` 5.0))

(event `self.ReceiveActorBeginOverlap`
  (params (OtherActor :type "Actor Object Reference"))
  (bind _returnvalue (`self.K2_GetActorLocation`))
  (`GameplayStatics.ApplyDamage` OtherActor 10.0 (`GameplayStatics.GetPlayerController` 0) self)
  (`GameplayStatics.SpawnSoundAtLocation` "/Game/StarterContent/Audio/Explosion_Cue.Explosion_Cue" _returnvalue (struct) 1.0 1.0 0.0 null null)
  (`GameplayStatics.SpawnEmitterAtLocation` "/Game/StarterContent/Particles/P_Explosion.P_Explosion" _returnvalue)
  (bind _asbp_game_mode (cast `/Game/P_38Game/BP_GameMode` (`GameplayStatics.GetGameMode`)))
  (`/Game/P_38Game/BP_GameMode.GameCheak` _asbp_game_mode)
  (`self.K2_DestroyActor`))

(fn `UserConstructionScript`)